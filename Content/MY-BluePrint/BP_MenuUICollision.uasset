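; BP_MenuUICollision is an in-world main menu screen with clickable Start and Quit components.
; A dynamic material instance on mesh slot 4 draws the display, with scalar parameters for hover highlights, flash and screen changes.
; Start plays a timeline flash, staggered screen glitch and sounds, then calls StartGameSequence on My_GameStateBase and disables hover feedback.
; Quit only plays a click sound, while Reset restores the screen and hover feedback.
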(event `self.ReceiveBeginPlay`
  (bind _returnvalue (`KismetMaterialLibrary.CreateDynamicMaterialInstance` "/Game/场景/Materials/MI_Display_Custom_Menu.MI_Display_Custom_Menu"))
  (bind _output_get (set `self.SelectMaterial` _returnvalue))
  (`PrimitiveComponent.SetMaterial` (`self.StaticMeshComponent`) 4 _output_get))

(event `self.StartGameButton.OnBeginCursorOver`
  (params (TouchedComponent :type "PrimitiveComponent Object Reference"))
  (bind _audio (`self.Audio`))
  (if (not (`self.Is StartGame`))
    (`MaterialInstanceDynamic.SetScalarParameterValue` (`self.SelectMaterial`) "PlayButtonAlpha" 1.0)
    (set `AudioComponent.Sound` (`self.Audio_OverLap`) _audio :!label _label)
    (`AudioComponent.Play` _audio 0.0)))

(event `self.StartGameButton.OnEndCursorOver`
  (params (TouchedComponent :type "PrimitiveComponent Object Reference"))
  (if (not (`self.Is StartGame`))
    (`MaterialInstanceDynamic.SetScalarParameterValue` (`self.SelectMaterial`) "PlayButtonAlpha" 0.0)))

(event `self.StartGameButton.OnClicked`
  (params (TouchedComponent :type "PrimitiveComponent Object Reference") (ButtonPressed :type "Key Structure"))
  (bind _selectmaterial (`self.SelectMaterial`))
  (bind _audio (`self.Audio`))
  (set `AudioComponent.Sound` (`self.Audio_Click_Start`) _audio)
  (`|ExecutionSequence`
    (:`then_0`
      (bind (_direction `_新建轨道_0`) (`Timeline|时间轴_0` :!via `PlayFromStart`)
        (:`Update`
          (`MaterialInstanceDynamic.SetScalarParameterValue` _selectmaterial "FlashAlpha" (* `_新建轨道_0` 0.05)))))
    (:`then_1`
      (`KismetSystemLibrary.Delay` 0.5)
      (`MaterialInstanceDynamic.SetScalarParameterValue` _selectmaterial "ScreenChange" 0.3)
      (`GameplayStatics.PlaySoundAtLocation` "/Game/MY-Audio/故障音效.故障音效" (0.0 0.0 0.0) (struct) 1.0 1.0 0.0 null null null)
      (`KismetSystemLibrary.Delay` 0.5)
      (`MaterialInstanceDynamic.SetScalarParameterValue` _selectmaterial "ScreenChange" 0.1))
    (:`then_2`
      (`AudioComponent.Play` _audio 0.0))
    (:`then_3`
      (`KismetSystemLibrary.Delay` 1.0)
      (bind _asmy_game_state_base (cast `/Game/MY-BluePrint/My_GameStateBase` (`GameplayStatics.GetGameState`)))
      (`/Game/MY-BluePrint/My_GameStateBase.StartGameSequence` _asmy_game_state_base)
      (set `self.Is StartGame` true))))

(event `self.QuitGameButton.OnBeginCursorOver`
  (params (TouchedComponent :type "PrimitiveComponent Object Reference"))
  (if (not (`self.Is StartGame`))
    (`MaterialInstanceDynamic.SetScalarParameterValue` (`self.SelectMaterial`) "QuitButtonAlpha" 1.0)
    (goto _label)))

(event `self.QuitGameButton.OnClicked`
  (params (TouchedComponent :type "PrimitiveComponent Object Reference") (ButtonPressed :type "Key Structure"))
  (bind _audio (`self.Audio`))
  (set `AudioComponent.Sound` (`self.Audio_Click_Quit`) _audio)
  (`AudioComponent.Play` _audio 0.0))

(event `self.QuitGameButton.OnEndCursorOver`
  (params (TouchedComponent :type "PrimitiveComponent Object Reference"))
  (if (not (`self.Is StartGame`))
    (`MaterialInstanceDynamic.SetScalarParameterValue` (`self.SelectMaterial`) "QuitButtonAlpha" 0.0)))

(event `Reset`
  (bind _selectmaterial (`self.SelectMaterial`))
  (`MaterialInstanceDynamic.SetScalarParameterValue` _selectmaterial "ScreenChange" 1.0)
  (`MaterialInstanceDynamic.SetScalarParameterValue` _selectmaterial "FlashAlpha" 0.0)
  (set `self.Is StartGame` false))

(fn `UserConstructionScript`)