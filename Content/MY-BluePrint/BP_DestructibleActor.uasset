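; Destructible prop actor that shatters once when its DestoryDamage event is called, then removes itself.
; The construction script applies the chosen destructible mesh when it differs from the current one and gives each material slot a dynamic instance.
; The event applies damage as an impulse along the hit direction, then a timeline drives the materials' Alpha parameter before the actor is destroyed.
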(event `self.ReceiveBeginPlay`)

(event `self.ReceiveTick`
  (params (DeltaSeconds :type "Float (single-precision)")))

(event `DestoryDamage`
  (params (Damage :type "Float (double-precision)") (`Hit Direction` :type "Vector Structure"))
  (bind _destrucible_actor (`self.Destrucible Actor`))
  ;[1 1 1] 破碎
  (if (`self.Can Destory`)
    (`DestructibleComponent.ApplyDamage` _destrucible_actor Damage (`SceneComponent.K2_GetComponentLocation` _destrucible_actor) `Hit Direction` Damage)
    (set `self.Can Destory` false)
    (bind (_direction _alpha) (`Timeline|Timeline_0` :!via `PlayFromStart`)
      (:`Update`
        (`MeshComponent.SetScalarParameterValueOnMaterials` (`self.Destrucible Actor`) "Alpha" _alpha))
      (:`Finished`
        (`self.K2_DestroyActor`)))))

(fn `UserConstructionScript`
  (bind _destrucible_actor (`self.Destrucible Actor`))
  (bind _destrucibleprefab (`self.DestruciblePrefab`))
  (bind _returnvalue (`DestructibleComponent.GetDestructibleMesh` _destrucible_actor))
  (if (!= _returnvalue _destrucibleprefab)
    (`DestructibleComponent.SetDestructibleMesh` _destrucible_actor _destrucibleprefab)
    (for (_array_element _array_index) (`SkeletalMesh.Materials` _destrucibleprefab)
      (bind _returnvalue_2 (`KismetMaterialLibrary.CreateDynamicMaterialInstance` (break `SkeletalMaterial` _array_element)))
      (`PrimitiveComponent.SetMaterial` _destrucible_actor _array_index _returnvalue_2))))