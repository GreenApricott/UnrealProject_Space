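; BP_Key is a key pickup actor that gives the player a key when touched.
; When its sphere is overlapped by the player pawn (a myActor) that lacks a key, it sets that pawn's HaveKey flag, plays a pickup sound and hides the Key component.
; It waits briefly before destroying itself, and ignores a player who already has a key.
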(event `self.Sphere.OnComponentBeginOverlap`
  (params (OverlappedComponent :type "PrimitiveComponent Object Reference") (OtherActor :type "Actor Object Reference") (OtherComp :type "PrimitiveComponent Object Reference") (OtherBodyIndex :type Integer) (bFromSweep :type Boolean) (SweepResult :type "HitResult Structure (by ref)"))
  (bind _asmy_actor (cast `/Game/MY-actor/myActor` (`GameplayStatics.GetPlayerPawn` 0)))
  (if (== _asmy_actor OtherActor)
    (if (not (`/Game/MY-actor/myActor.Have Key` _asmy_actor))
      (set `/Game/MY-actor/myActor.Have Key` true _asmy_actor)
      (`AudioComponent.Play` (`self.Audio_PickUp_key`) 0.0)
      (`SceneComponent.SetVisibility` (`self.Key`) false false)
      (`KismetSystemLibrary.Delay` 1.0)
      (`self.K2_DestroyActor`))))

(fn `UserConstructionScript`)