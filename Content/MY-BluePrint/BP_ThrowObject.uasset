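; BP_ThrowObject is a timed explosive prop that detonates after a delay from spawn, then destroys itself.
; Detonation spawns a Niagara effect and sound, then applies fixed damage and an outward hit direction to GameState-listed destructible actors within explosion range.
; Mesh hits enable physics simulation if it is off and play an impact sound, throttled by a DoOnce reset after a short random delay.
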(event `self.ReceiveBeginPlay`
  (bind _explosion_damage (`self.Explosion Damage`))
  (bind _returnvalue (`SceneComponent.K2_GetComponentLocation` (`self.StaticMesh`)))
  (bind _returnvalue_2 (`KismetMathLibrary.MakeVector` (.x (`SceneComponent.K2_GetComponentLocation` (`self.StaticMesh`))) (.y (`SceneComponent.K2_GetComponentLocation` (`self.StaticMesh`))) (+ (.z (`SceneComponent.K2_GetComponentLocation` (`self.StaticMesh`))) 10.0)))
  (`KismetSystemLibrary.Delay` (`self.Time To Explosive`))
  (`|ExecutionSequence`
    (:`then_0`
      ;[1 1 1] 爆炸 特效
      (`NiagaraFunctionLibrary.SpawnSystemAtLocation` "/Game/MY-Niagara/N_Explosion.N_Explosion" _returnvalue_2 (struct) (2.0 2.0 2.0) true true "AutoRelease")
      (`GameplayStatics.PlaySoundAtLocation` "/Game/StarterContent/Audio/Explosion02.Explosion02" _returnvalue_2 (struct) 1.0 1.0 0.0 null null null)
      (`KismetSystemLibrary.PrintString` "爆炸！"))
    (:`then_1`
      ;[1 1 1] 遍历爆炸物
      (bind _asmy_game_state_base (cast `/Game/MY-BluePrint/My_GameStateBase` (`GameplayStatics.GetGameState`)))
      (for _array_element (`/Game/MY-BluePrint/My_GameStateBase.Destructible Actors` _asmy_game_state_base)
        (bind _returnvalue_3 (`SceneComponent.K2_GetComponentLocation` (`/Game/MY-BluePrint/BP_DestructibleActor.Destrucible Actor` _array_element)))
        (if (<= (`KismetMathLibrary.Vector_Distance` _returnvalue_3 _returnvalue) (`self.Explosion Range`))
          (`/Game/MY-BluePrint/BP_DestructibleActor.DestoryDamage` _array_element _explosion_damage (* (`KismetMathLibrary.Normal` (- _returnvalue_3 _returnvalue)) _explosion_damage)))))
    (:`then_2`
      (`self.K2_DestroyActor`))))

(event `self.StaticMesh.OnComponentHit`
  (params (HitComponent :type "PrimitiveComponent Object Reference") (OtherActor :type "Actor Object Reference") (OtherComp :type "PrimitiveComponent Object Reference") (NormalImpulse :type "Vector Structure") (Hit :type "HitResult Structure (by ref)"))
  (bind _staticmesh (`self.StaticMesh`))
  ;[1 1 1] 碰撞音效
  (`|ExecutionSequence`
    (:`then_0`
      (if (not (`SceneComponent.IsAnySimulatingPhysics` _staticmesh))
        (`PrimitiveComponent.SetSimulatePhysics` _staticmesh true)))
    (:`then_1`
      (`/Engine/EditorBlueprintResources/StandardMacros.DoOnce` false :!label _label
        (:`Completed`
          (bind _returnvalue (`GameplayStatics.SpawnSoundAtLocation` (`self.Hit Sounds`) Hit_Location (struct) 0.5 1.0 0.0 null null))
          (set `AudioComponent.PitchModulationMin` 0.4 _returnvalue)
          (set `AudioComponent.PitchModulationMax` 0.6 _returnvalue))))
    (:`then_2`
      (`KismetSystemLibrary.Delay` (`KismetMathLibrary.RandomFloatInRange` 0.2 0.4))
      (goto _label :!via `Reset`))))

(fn `UserConstructionScript`)