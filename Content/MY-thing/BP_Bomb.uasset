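; Reusable bomb that the player picks up and drops with E, then detonates with R when nearby.
; Tick polls distance and myActor input flags to update the prompt billboard and snap the held bomb to the "aim" socket.
; After a fuse delay, it spawns effects and applies directional damage to in-range DestructibleActors from My_GameStateBase.
; It then hides and respawns at the RespawnBombPos actor's location; physics hits play throttled impact sounds.
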(event `self.ReceiveBeginPlay`
  (bind _asmy_actor (cast `/Game/MY-actor/myActor` (`GameplayStatics.GetPlayerCharacter` 0)))
  (set `self.BP_Player` _asmy_actor)
  (bind _returnvalue (`GameplayStatics.GetActorOfClass` "/Game/MY-BluePrint/RespawnBombPos.RespawnBombPos_C"))
  (`/Engine/EditorBlueprintResources/StandardMacros.IsValid` _returnvalue
    (:`Is Valid`
      (set `self.RespawnPos` (`SceneComponent.K2_GetComponentLocation` (`/Game/MY-BluePrint/RespawnBombPos.DefaultSceneRoot` _returnvalue))))
    (:`Is Not Valid`
      (set `self.RespawnPos` (0.0 0.0 0.0)))))

(event `self.ReceiveTick`
  (params (DeltaSeconds :type "Float (single-precision)"))
  (`self.Set UI`)
  (`self.Check Player`)
  (`self.Set Bomb`)
  (`self.Detonate`))

(event `Check Player`
  ;[1 1 1] 炸弹距离检测
  (set `self.Is Player Near` (<= (`KismetMathLibrary.Vector_Distance` (`self.K2_GetActorLocation` (`GameplayStatics.GetPlayerCharacter` 0)) (`SceneComponent.K2_GetComponentLocation` (`self.Bomb`))) (`self.Min Distance To Player`))))

(event `Set UI`
  (bind _materialbillboard (`self.MaterialBillboard`))
  (bind _returnvalue (and (`self.Can Pick Up`) (== (not (`self.Is Holding`)) (`self.Is Player Near`))))
  ;[1 1 1] 设置UI 可视化 和 位置
  (`SceneComponent.SetVisibility` _materialbillboard _returnvalue false)
  (if _returnvalue
    (`SceneComponent.K2_SetWorldLocation` _materialbillboard (+ (`SceneComponent.K2_GetComponentLocation` (`self.Bomb`)) (`self.UI Offset`)) false false)))

(event `Set Bomb`
  (bind _bp_player (`self.BP_Player`))
  (bind _bomb (`self.Bomb`))
  (bind _is_holding (`self.Is Holding`))
  (bind _is_e (`/Game/MY-actor/myActor.Is E` _bp_player))
  ;[1 1 1] 设置炸弹 可视化 和 位置
  (set `/Game/MY-actor/myActor.Is Holding` _is_holding _bp_player) ; 设置人物动画
  (`SceneComponent.SetVisibility` (`self.Bomb`) (and (not _is_holding) (not (`self.Is Respawning`))) false)
  (if _is_holding
    (if _is_e
      ;;[1 1 1] 扔掉炸弹
      (set `self.Is Holding` false)
      (set `/Game/MY-actor/myActor.Is E` false _bp_player)
      (set `/Game/MY-actor/myActor.Pick Actor` null _bp_player)
      (else
        ;;[1 1 1] 炸弹 在玩家身上
        (`PrimitiveComponent.SetCollisionEnabled` _bomb "NoCollision")
        (`SceneComponent.K2_SetWorldLocation` _bomb (`SceneComponent.GetSocketLocation` (`Actor.RootComponent` (`GameplayStatics.GetPlayerCharacter` 0)) "aim") false false)
        (set `/Game/MY-actor/myActor.Pick Actor` self _bp_player)))
    (else
      ;;[1 1 1] 炸弹 不在玩家身上
      (`PrimitiveComponent.SetCollisionEnabled` (`self.Bomb`) "PhysicsOnly")
      (if (and (`self.Can Pick Up`) (and (`self.Is Player Near`) _is_e))
        (set `self.Is Holding` true)
        (set `/Game/MY-actor/myActor.Is E` false _bp_player)
        (`/Game/MY-actor/myActor.Audio_Get` _bp_player)))))

(event `Detonate`
  (bind _explosion_damage (`self.Explosion Damage`))
  (bind _returnvalue (`SceneComponent.K2_GetComponentLocation` (`self.Bomb`)))
  (bind _returnvalue_2 (`KismetMathLibrary.MakeVector` (.x (`SceneComponent.K2_GetComponentLocation` (`self.Bomb`))) (.y (`SceneComponent.K2_GetComponentLocation` (`self.Bomb`))) (+ (.z (`SceneComponent.K2_GetComponentLocation` (`self.Bomb`))) 10.0)))
  ;[1 1 1] 可爆炸检测
  (bind _asmy_actor (cast `/Game/MY-actor/myActor` (`GameplayStatics.GetPlayerCharacter` 0)))
  (if (`self.Is Player Near`)
    (if (`self.Is Holding`)
      _
      (elif (`/Game/MY-actor/myActor.Is R` _asmy_actor)
        (set `self.Can Pick Up` false) ; 不能再捡起
        (`KismetSystemLibrary.Delay` (`self.Time To Explosive`))
        (`|ExecutionSequence`
          (:`then_0`
            ;[1 1 1] 爆炸 特效
            (`NiagaraFunctionLibrary.SpawnSystemAtLocation` "/Game/MY-Niagara/N_Explosion.N_Explosion" _returnvalue_2 (struct) (2.0 2.0 2.0) true true "AutoRelease")
            (`GameplayStatics.PlaySoundAtLocation` "/Game/StarterContent/Audio/Explosion02.Explosion02" _returnvalue_2 (struct) 1.0 1.0 0.0 null null null)
            (`KismetSystemLibrary.PrintString` "爆炸！"))
          (:`then_1`
            ;[1 1 1] 遍历爆炸物
            (bind _asmy_game_state_base (cast `/Game/MY-BluePrint/My_GameStateBase` (`GameplayStatics.GetGameState`)))
            (for _array_element (`/Game/MY-BluePrint/My_GameStateBase.Destructible Actors` _asmy_game_state_base)
              (bind _returnvalue_3 (`SceneComponent.K2_GetComponentLocation` (`/Game/MY-BluePrint/BP_DestructibleActor.Destrucible Actor` _array_element)))
              (if (<= (`KismetMathLibrary.Vector_Distance` _returnvalue_3 _returnvalue) (`self.Explosion Range`))
                (`/Game/MY-BluePrint/BP_DestructibleActor.DestoryDamage` _array_element _explosion_damage (* (`KismetMathLibrary.Normal` (- _returnvalue_3 _returnvalue)) _explosion_damage)))))
          (:`then_2`
            (`self.Throw Out`)))))))

(event `self.Bomb.OnComponentHit`
  (params (HitComponent :type "PrimitiveComponent Object Reference") (OtherActor :type "Actor Object Reference") (OtherComp :type "PrimitiveComponent Object Reference") (NormalImpulse :type "Vector Structure") (Hit :type "HitResult Structure (by ref)"))
  ;[1 1 1] 音效
  (if (not (`self.Is Respawning`))
    (`|ExecutionSequence`
      (:`then_0`
        (`/Engine/EditorBlueprintResources/StandardMacros.DoOnce` false :!label _label
          (:`Completed`
            (bind _returnvalue (`GameplayStatics.SpawnSoundAtLocation` (`self.Hit Sound`) Hit_Location (struct) 0.5 1.0 0.0 null null))
            (set `AudioComponent.PitchModulationMin` 0.4 _returnvalue)
            (set `AudioComponent.PitchModulationMax` 0.6 _returnvalue))))
      (:`then_1`
        (`KismetSystemLibrary.Delay` (`KismetMathLibrary.RandomFloatInRange` 0.2 0.4))
        (goto _label :!via `Reset`)))))

(event `Throw Out`
  (bind _bomb (`self.Bomb`))
  (bind _bp_player (`self.BP_Player`))
  ;[1 1 1] 扔出炸弹
  (set `self.Is Holding` false)
  (set `/Game/MY-actor/myActor.Is E` false _bp_player)
  (set `/Game/MY-actor/myActor.Pick Actor` null _bp_player)
  (set `self.Can Pick Up` false)
  (set `self.Is Respawning` true)
  (`KismetSystemLibrary.Delay` 3.0)
  (`SceneComponent.K2_SetWorldLocation` _bomb (`self.RespawnPos`) false false)
  (`SceneComponent.SetVisibility` _bomb true false)
  (set `self.Can Pick Up` true)
  (set `self.Is Respawning` false))

(fn `UserConstructionScript`)